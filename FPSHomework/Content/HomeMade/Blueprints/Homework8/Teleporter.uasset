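; Teleporter actor that sends anything entering its Box trigger to a linked teleporter referenced by TeleportTo.
; Overlap stores the actor and waits DelayTimer seconds; leaving the box clears the stored actor, cancelling the transfer.
; After the delay, the linked teleporter's TeleportPlayer moves the actor to its own Billboard location with zeroed rotation.
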(event `self.Box.OnComponentBeginOverlap`
  (params (OverlappedComponent :type "PrimitiveComponent Object Reference") (OtherActor :type "Actor Object Reference") (OtherComp :type "PrimitiveComponent Object Reference") (OtherBodyIndex :type Integer) (bFromSweep :type Boolean) (SweepResult :type "HitResult Structure (by ref)"))
  (set `self.ActorToTransport` OtherActor)
  (`KismetSystemLibrary.Delay` (`self.DelayTimer`))
  (bind _actortotransport (`self.ActorToTransport`)
    (:`then`
      (bind _teleportto (`self.TeleportTo`)
        (:`then`
          (`self.TeleportPlayer` _teleportto _actortotransport))
        (:`else`)))
    (:`else`)))

(event `self.Box.OnComponentEndOverlap`
  (params (OverlappedComponent :type "PrimitiveComponent Object Reference") (OtherActor :type "Actor Object Reference") (OtherComp :type "PrimitiveComponent Object Reference") (OtherBodyIndex :type Integer))
  (set `self.ActorToTransport` null))

(fn `TeleportPlayer`
  (params (Actor :type "Actor Object Reference"))
  (`self.K2_TeleportTo` :`self` Actor :`DestLocation` (`SceneComponent.K2_GetComponentLocation` (`self.Billboard`))))

(fn `UserConstructionScript`)