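; Spawner actor that builds a line, plane or cuboid of BP_SphereForSpawning child actors in its construction script.
; A dimension setting drives a MultiGate that collapses unused axis sizes to one, then nested loops add the spheres.
; SpacingFunction offsets each by index, bounds and SphereSpacing, while a FlipFlop shifts alternate Z layers along Y.
; Each sphere's grid position sets its RGB colour, producing a gradient.
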(fn `SpacingFunction`
  (params (Axis :type "Float (double-precision)") (Index :type Integer) (Spacing :type "Float (double-precision)"))
  (returns (ReturnValue :type "Float (double-precision)"))
  (locals (SphereSpacing :type "Float (double-precision)"))
  ;[1 1 1] dictates the spacing of the spheres in a row
  (set `local.SphereSpacing` Spacing)
  (return (* (* Index (* (* Axis 2.0) (`local.SphereSpacing`))) (`local.SphereSpacing`))))

(fn `UserConstructionScript`
  (locals (ChildSphere :type "ChildActorComponent Object Reference") (ZSize :type Integer :default 5) (XSize :type Integer :default 5) (YSize :type Integer :default 5) (SphereSpacing :type "Float (double-precision)" :default 1.0) (LocalIndexZ :type Integer) (LocalIndexX :type Integer) (LocalIndexY :type Integer) (ExtraYSpace :type "Float (double-precision)" :default 100.0) (ExtraXSpace :type "Float (double-precision)" :default 100.0))
  (bind _childsphere (`local.ChildSphere`))
  (bind (_origin _boxextent) (`self.GetActorBounds` (`ChildActorComponent.ChildActor` (`local.ChildSphere`)) true))
  ;[1 1 1] Controls the number of dimensions to the cuboid of spheres
  (`|MultiGate` false false (select `/Game/HomeMade/Blueprints/HomeWork7/SpawnerDimensions` (`self.DimensionsNo.`) :`NewEnumerator0` 3 :`NewEnumerator2` 1 :`NewEnumerator3` 2)
    (:`Out 0`
      (set `local.ZSize` 1)
      (set `local.XSize` 1))
    (:`Out 1`
      (set `local.ZSize` 1))
    (:`Out 2`
      _)
    (:`Out 3`
      (set `local.ZSize` 1)
      (set `local.XSize` 1)
      (set `local.YSize` 1)))
  ;[1 1 1] Creates a 3 dimensional cuboid of spheres the dimensions of which are dictated by Zsize, Xsize and Ysize variables
  (for _index (range (`local.ZSize`))
    ;;[1 1 1] Offsets every second row by 50 to create a tiling effect
    (`/Engine/EditorBlueprintResources/StandardMacros.FlipFlop`
      (:`A`
        (set `local.ExtraYSpace` 0.0))
      (:`B`
        (set `local.ExtraYSpace` 50.0)))
    (for _index_2 (range (`local.XSize`))
      (for _index_3 (range (`local.YSize`))
        (set `local.LocalIndexZ` _index)
        (set `local.LocalIndexX` _index_2)
        (set `local.LocalIndexY` _index_3)
        (bind _returnvalue (`AddComponent|NODE_AddChildActorComponent-0`))
        (set `local.ChildSphere` _returnvalue)
        (`ChildActorComponent.SetChildActorClass` _childsphere "/Game/HomeMade/Blueprints/HomeWork3/BP_SphereForSpawning.BP_SphereForSpawning_C")
        (`SceneComponent.K2_AddLocalOffset` _childsphere (`KismetMathLibrary.MakeVector` (`self.SpacingFunction` (.x _boxextent) (`local.LocalIndexX`) (`local.SphereSpacing`)) (+ (`self.SpacingFunction` (.y _boxextent) (`local.LocalIndexY`) (`local.SphereSpacing`)) (`local.ExtraYSpace`)) (`self.SpacingFunction` (.z _boxextent) (`local.LocalIndexZ`) (`local.SphereSpacing`))) false false)
        (bind _asbp_sphere_for_spawning (cast `/Game/HomeMade/Blueprints/HomeWork3/BP_SphereForSpawning` (`ChildActorComponent.ChildActor` (`local.ChildSphere`))))
        ;;[1 1 1] changes the colour of the spheres as each is created, to create a colour gradient effect
        (`/Game/HomeMade/Blueprints/HomeWork3/BP_SphereForSpawning.SetColour` _asbp_sphere_for_spawning (make `LinearColor` (/ (`KismetMathLibrary.Conv_IntToDouble` (+ (`local.LocalIndexZ`) 1)) (`KismetMathLibrary.Conv_IntToDouble` (`local.ZSize`))) (/ (`KismetMathLibrary.Conv_IntToDouble` (+ (`local.LocalIndexX`) 1)) (`KismetMathLibrary.Conv_IntToDouble` (`local.XSize`))) (/ (`KismetMathLibrary.Conv_IntToDouble` (+ (`local.LocalIndexY`) 1)) (`KismetMathLibrary.Conv_IntToDouble` (`local.YSize`)))))))))