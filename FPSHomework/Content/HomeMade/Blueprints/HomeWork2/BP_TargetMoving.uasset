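; BP_TargetMoving is a target actor whose cube slides back and forth along the world Y axis.
; Tick moves the cube by a delta-scaled speed while a limit counter drops once per frame, flipping direction and resetting at zero.
; BeginPlay sets a half-length first leg because the cube starts mid-path.
; Because the counter counts frames rather than time, travel distance varies with frame rate.
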(event `self.ReceiveBeginPlay`
  ;[1 1 1] first movement is only half because it starts halfway
  (`parent.ReceiveBeginPlay`)
  (set `self.OffsetLimit` 200.0)
  (set `self.OffsetSpeed` 300.0))

(event `self.ReceiveTick`
  (params (DeltaSeconds :type "Float (single-precision)"))
  (bind _offsetspeed (`self.OffsetSpeed`))
  (bind _offsetlimit (`self.OffsetLimit`))
  (`parent.ReceiveTick` DeltaSeconds)
  ;[1 1 1] Drifts slowly back and fourth across a set distance(offsetLimit)
  ; the starting position is halfway
  (`SceneComponent.K2_AddWorldOffset` (`self.Cube`) (`KismetMathLibrary.MakeVector` 0.0 (* DeltaSeconds _offsetspeed)) false false)
  (set `self.OffsetLimit` (- _offsetlimit 1.0))
  (if (<= _offsetlimit 0.0)
    (set `self.OffsetSpeed` (* _offsetspeed -1.0))
    (set `self.OffsetLimit` 400.0)))

(fn `UserConstructionScript`
  (`parent.UserConstructionScript`))