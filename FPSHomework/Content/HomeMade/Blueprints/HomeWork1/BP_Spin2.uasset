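; BP_Spin2 is an actor that continuously spins a centre cube and its Top, Bottom, Left and Right cubes.
; BeginPlay sets SpinSpeed, and Tick passes it with delta time to HandleSpinning for frame-rate-independent local rotation.
; The centre Cube pitches at half speed to spin the whole assembly.
; Top and Bottom roll in opposite directions, while Left and Right yaw in opposite directions, at full speed.
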(event `self.ReceiveTick`
  (params (DeltaSeconds :type "Float (single-precision)"))
  (`self.HandleSpinning` DeltaSeconds (stale `self.ReceiveBeginPlay` _output_get)))

(event `self.ReceiveBeginPlay`
  ;[1 1 1] sets the initial Spin Speed
  (bind _output_get (set `self.SpinSpeed` 100.0)))

(fn `HandleSpinning`
  (params (delta :type "Float (double-precision)") (SpinSpeed :type "Float (double-precision)"))
  (bind _returnvalue (* delta SpinSpeed))
  (bind _returnvalue_2 (* _returnvalue -1.0))
  ;[1 1 1] Spins the entire cube
  (`SceneComponent.K2_AddLocalRotation` (`self.Cube`) (`KismetMathLibrary.MakeRotator` 0.0 (/ _returnvalue 2.0)) false false)
  ;[1 1 1] make each cube spin away from centre cube
  (`SceneComponent.K2_AddLocalRotation` (`self.top`) (`KismetMathLibrary.MakeRotator` _returnvalue_2) false false)
  (`SceneComponent.K2_AddLocalRotation` (`self.right`) (`KismetMathLibrary.MakeRotator` 0.0 0.0 _returnvalue_2) false false)
  (`SceneComponent.K2_AddLocalRotation` (`self.left`) (`KismetMathLibrary.MakeRotator` 0.0 0.0 _returnvalue) false false)
  (`SceneComponent.K2_AddLocalRotation` (`self.bottom`) (`KismetMathLibrary.MakeRotator` _returnvalue) false false))

(fn `UserConstructionScript`)